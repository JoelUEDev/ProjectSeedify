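; AC_Interaction is an actor component that handles player interaction with collectable items and the related on-screen notifications.
; On BeginPlay it creates input-prompt and collection-notification widgets and adds both to the viewport.
; An availability event passes the interactable and its type to the prompt, depending on visibility.
; CollectItem queries the referenced actor, shows item information if uncollected, then informs that actor of collection by the component's owner.
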(event `self.ReceiveBeginPlay`
  ;[1 0 0] Begin Play
  ;[1 1 1] Widget Setup
  (bind _returnvalue (`|CreateWidget` "/Game/DemoCase/Blueprints/Widget/HUD/WB_InputNotification.WB_InputNotification_C"))
  (bind _output_get (set `self.Widget: Notification` _returnvalue))
  (`UserWidget.AddToViewport` _output_get 0)
  (bind _returnvalue_2 (`|CreateWidget` "/Game/DemoCase/Blueprints/Widget/Notification/BW_Notification.BW_Notification_C"))
  (bind _output_get_2 (set `self.Widget: Collection Notifcation` _returnvalue_2))
  (`UserWidget.AddToViewport` _output_get_2 0))

(event `Event Notification: Interaction Available`
  (params (`Actor Reference` :type "Actor Object Reference") (`Visible?` :type Boolean) (`Interaction Type` :type "/Game/DemoCase/Data/Enum/E_InteractionType Enum" :default "NewEnumerator0"))
  ;[1 0 0] Interactable In Range
  ;[1 1 1] Input Notification For Player If Interaction is Available
  (bind _output_get (set `self.Actor Reference` (select `bool` `Visible?` :`true` `Actor Reference`)))
  (`/Game/DemoCase/Blueprints/Widget/HUD/WB_InputNotification.Interaction Available` (`self.Widget: Notification`) _output_get `Interaction Type`))

(event `Event Collect Item`
  (bind _actor_reference (`self.Actor Reference`))
  ;[1 0 0] Interactable Collected
  ;[1 1 1] If Actor Reference Is Valid, Display Notification To Player Of Collection and Inform BP_Interactable It Has Been Collected
  (`/Engine/EditorBlueprintResources/StandardMacros.IsValid` _actor_reference
    (:`Is Valid`
      (bind (_item_information _collected) (message `/Game/DemoCase/Data/Interface/BI_Interactable.GetItemInformation` _actor_reference))
      (if (not _collected)
        (`/Game/DemoCase/Blueprints/Widget/Notification/BW_Notification.NotificationUpdate` (`self.Widget: Collection Notifcation`) _item_information)
        (message `/Game/DemoCase/Data/Interface/BI_Interactable.ItemCollected` _actor_reference (`self.GetOwner`))))))