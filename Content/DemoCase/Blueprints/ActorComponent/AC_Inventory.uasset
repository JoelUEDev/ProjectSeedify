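; Actor component that manages the player's inventory UI.
; On begin play it creates a WB_Inventory widget and keeps a reference to it.
; OpenInventory uses a FlipFlop to toggle the widget in the viewport while pausing and unpausing the game.
; ItemAddedToInventory forwards item info to the widget, which handles adding the entry.
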(event `self.ReceiveBeginPlay`
  ;[1 0 0] Begin Play
  ;[1 1 1] Widget Setup
  (bind _returnvalue (`|CreateWidget` "/Game/DemoCase/Blueprints/Widget/Inventory/WB_Inventory.WB_Inventory_C"))
  (set `self.Widget:Inventory` _returnvalue))

(event `Event Open Inventory`
  (bind _widget_inventory (`self.Widget:Inventory`))
  ;[1 0 0] Open Inventory
  ;[1 1 1] Open/Close Inventory Widget
  (`/Engine/EditorBlueprintResources/StandardMacros.FlipFlop`
    (:`A`
      (`GameplayStatics.SetGamePaused` true)
      (`UserWidget.AddToViewport` _widget_inventory 0))
    (:`B`
      (`GameplayStatics.SetGamePaused` false)
      (`Widget.RemoveFromParent` _widget_inventory))))

(event `Event Item Added To Inventory`
  (params (`Item Info` :type "/Game/DemoCase/Data/Struct/S_ItemInformation Structure"))
  ;[1 0 0] Item Added
  ;[1 1 1] Update Inventory With Child Widget
  (`/Game/DemoCase/Blueprints/Widget/Inventory/WB_Inventory.Event Add Item To Inventory` (`self.Widget:Inventory`) `Item Info`))