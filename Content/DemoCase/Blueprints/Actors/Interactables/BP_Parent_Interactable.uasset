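; BP_Parent_Interactable is a parent actor for collectable items that the player picks up into an inventory.
; Construction looks up its item name in DT_ItemInfo and applies the item image to both image planes through dynamic materials.
; Range overlaps notify the other actor's AC_Interaction component of availability.
; On collection, it flags itself collected and, only once, passes its item info to the collector's AC_Inventory and calls PlayerDesiresToCollect.
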(event `self.Range - Collectable.OnComponentBeginOverlap`
  (params (OverlappedComponent :type "PrimitiveComponent Object Reference") (OtherActor :type "Actor Object Reference") (OtherComp :type "PrimitiveComponent Object Reference") (OtherBodyIndex :type Integer) (bFromSweep :type Boolean) (SweepResult :type "HitResult Structure (by ref)"))
  (bind _returnvalue (`self.GetComponentByClass` OtherActor "/Game/DemoCase/Blueprints/ActorComponent/AC_Interaction.AC_Interaction_C"))
  ;[1 0 0] Overlap: Collectable Range
  ;[1 1 1] Send Overlap Notification Message Directly To Player AC_Interaction If Valid
  (`/Engine/EditorBlueprintResources/StandardMacros.IsValid` _returnvalue
    (:`Is Valid`
      (`/Game/DemoCase/Blueprints/ActorComponent/AC_Interaction.Event Notification: Interaction Available` _returnvalue self true (`self.Interaction Type`)))))

(event `self.Range - Collectable.OnComponentEndOverlap`
  (params (OverlappedComponent :type "PrimitiveComponent Object Reference") (OtherActor :type "Actor Object Reference") (OtherComp :type "PrimitiveComponent Object Reference") (OtherBodyIndex :type Integer))
  (bind _returnvalue (`self.GetComponentByClass` OtherActor "/Game/DemoCase/Blueprints/ActorComponent/AC_Interaction.AC_Interaction_C"))
  ;[1 0 0] Overlap: Collectable Range
  ;[1 1 1] Send Overlap Notification Message Directly To Player AC_Interaction If Valid
  (`/Engine/EditorBlueprintResources/StandardMacros.IsValid` _returnvalue
    (:`Is Valid`
      (`/Game/DemoCase/Blueprints/ActorComponent/AC_Interaction.Event Notification: Interaction Available` _returnvalue self false "NewEnumerator0"))))

(event `/Game/DemoCase/Data/Interface/BI_Interactable.ItemCollected`
  (params (CollectedBy :type "Actor Object Reference"))
  ;[1 0 0] Upon Collected (This Actor)
  ;[1 1 1] Send Item Info Detail Directly To AC_Inventory Then Destroy This Actor
  (set `self.Collected` true)
  (`/Engine/EditorBlueprintResources/StandardMacros.DoOnce` false
    (:`Completed`
      (`/Game/DemoCase/Blueprints/ActorComponent/AC_Inventory.Event Item Added To Inventory` (`self.GetComponentByClass` CollectedBy "/Game/DemoCase/Blueprints/ActorComponent/AC_Inventory.AC_Inventory_C") (`self.ItemInfo`))
      (`self.PlayerDesiresToCollect`))))

(fn `GetItemInformation`
  (returns (`Item Information` :type "/Game/DemoCase/Data/Struct/S_ItemInformation Structure") (Collected :type Boolean))
  (return (`self.ItemInfo`) (`self.Collected`)))

(fn `UserConstructionScript`
  ;[1 1 1] Search Data Table For Item Information Based Upon Item Name Enum - Set Textures Accordingly
  (bind _returnvalue (`|GetDataTableRow` "/Game/DemoCase/Data/DataTable/DT_ItemInfo.DT_ItemInfo" (`KismetStringLibrary.Conv_StringToName` (`|GetEnumeratorNameAsString` (`self.ItemName`))))
    (:`then`
      (bind _output_get (set `self.ItemInfo` _returnvalue))
      (bind _returnvalue_2 (`PrimitiveComponent.CreateDynamicMaterialInstance` (`self.Plane - Image Side A`) 0 null "None"))
      (bind ((`Image_11_F0B5836946EF4D4CAB5DDF9F53308C1F` _image)) (break `/Game/DemoCase/Data/Struct/S_ItemInformation` _output_get))
      (`MaterialInstanceDynamic.SetTextureParameterValue` _returnvalue_2 "TextureBase" _image)
      (bind _returnvalue_3 (`PrimitiveComponent.CreateDynamicMaterialInstance` (`self.Plane - Image Side B`) 0 null "None"))
      (`MaterialInstanceDynamic.SetTextureParameterValue` _returnvalue_3 "TextureBase" _image))))