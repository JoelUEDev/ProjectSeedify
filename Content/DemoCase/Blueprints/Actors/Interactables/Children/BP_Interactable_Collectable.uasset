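; Collectable child interactable that visually disappears and removes itself from the world when the player collects it.
; On BeginPlay it binds to the player's collect event and creates dynamic material instances for every material slot on its static mesh.
; Collection plays the ItemDisappear timeline, which drives each material's Visibility parameter, then destroys the actor when finished.
; The material helper also accepts a skeletal mesh, preferring it when valid.
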(event `self.ReceiveBeginPlay`
  ;[1 0 0] Begin Play
  ;[1 1 1] Bind Event Upon This Actor Being Collected, Destroy Actor
  (add `self.PlayerDesiresToCollect` (delegate `Player Desires To Collect`))
  (`self.CreateMaterialInstances` (`self.StaticMesh`)))

(event `Player Desires To Collect`
  ;[1 0 0] Begin Play
  ;[1 1 1] Bind Event Upon This Actor Being Collected, Destroy Actor
  (bind (_direction _newtrack_0) (`Timeline|Item Disappear` :!via `PlayFromStart`)
    (:`Update`
      (for _array_element (`self.Dynamic Material Instances`)
        (`MaterialInstanceDynamic.SetScalarParameterValue` _array_element "Visibility" _newtrack_0)))
    (:`Finished`
      (`self.K2_DestroyActor`))))

(fn `CreateMaterialInstances`
  (params (Static :type "MeshComponent Object Reference") (Skeletal :type "SkeletalMeshComponent Object Reference"))
  (bind _returnvalue (select `bool` (`KismetSystemLibrary.IsValid` Skeletal) :`false` Static :`true` Skeletal :!type "MeshComponent Object Reference"))
  (bind _result (`/Engine/EditorBlueprintResources/StandardMacros.DecrementInt` (`KismetArrayLibrary.Array_Length` (`MeshComponent.GetMaterials` _returnvalue)))
    (:`  `
      (for _index (range (+ _result 1))
        (bind _returnvalue_2 (`PrimitiveComponent.CreateDynamicMaterialInstance` _returnvalue _index null "None"))
        (`KismetArrayLibrary.Array_Add` (`self.Dynamic Material Instances`) _returnvalue_2)))))

(fn `UserConstructionScript`
  (`parent.UserConstructionScript`))